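; BP_Ceiling is a tiled ceiling actor for the Batcave that builds a grid of mesh instances from Rows and Columns.
; The construction script runs nested loops that add local-space instances to TileInstance, spacing them along X and Y by the mesh's local bounds so tiles sit edge to edge.
; The event graph holds only disabled placeholder events, so there is no runtime logic.
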(fn `UserConstructionScript`
  (bind _tile_instance (`self.Tile_Instance`))
  (bind (_min _max) (`StaticMeshComponent.GetLocalBounds` _tile_instance))
  (bind (_returnvalue_x _returnvalue_y) (`KismetMathLibrary.BreakVector` (- _max _min)))
  (for _index (range (+ (`self.Rows`) 1))
    (for _index_2 (range (+ (`self.Columns`) 1))
      (`InstancedStaticMeshComponent.AddInstance` _tile_instance (`KismetMathLibrary.MakeTransform` (`KismetMathLibrary.MakeVector` (* _index _returnvalue_x) (* _index_2 _returnvalue_y))) false))))